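; Player-controlled kart pawn that extends its parent with driving input, camera control and gear-shift audio.
; Throttle, steering and camera-view toggle pass through CanMove, which continues only while the player controller's IsRacing is set.
; Each tick, GearSound slides a speed window to fake gears below a speed cap, playing a blow-off sound on upshifts.
; The Swoop event plays a timeline that rotates the spring arm and main camera.
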(event `self.ReceiveBeginPlay`
  (`parent.ReceiveBeginPlay`))

(event `self.ReceiveTick`
  (params (DeltaSeconds :type "Float (single-precision)"))
  (`parent.ReceiveTick` DeltaSeconds)
  (if (< (`self.Current Horizontal Speed`) 3500.0)
    (`|ExecutionSequence`
      (:`then_0`
        (if (< (`self.Current Horizontal Speed`) (`self.GearDown`))
          (set `self.GearDown` (- (`self.GearDown`) 1000.0))
          (set `self.GearUp` (- (`self.GearUp`) 1000.0))))
      (:`then_1`
        (if (> (`self.Current Horizontal Speed`) (`self.GearUp`))
          (set `self.GearDown` (+ (`self.GearDown`) 1000.0))
          (set `self.GearUp` (+ (`self.GearUp`) 1000.0))
          (`GameplayStatics.PlaySound2D` "/Game/Sound/Cue/SC_BlowOff.SC_BlowOff"))))))

(event `InputAxis|Forward`
  (params (AxisValue :type "Float (single-precision)"))
  (`self.CanMove`
    (:`Out`
      (`self.Set Throttle Input` (* AxisValue (`self.ThrottleMultiplier`))))))

(event `InputAxis|Steer`
  (params (AxisValue :type "Float (single-precision)"))
  (`self.CanMove`
    (:`Out`
      (`self.Set Steering Input` (* AxisValue (`self.SteerMultiplier`))))))

(event `InputAction|View`
  (params (Key :type "Key Structure"))
  (:`Pressed`
    (`self.CanMove`
      (:`Out`
        (`/Engine/EditorBlueprintResources/StandardMacros.FlipFlop`
          (:`A`
            (`ActorComponent.SetActive` (`self.Main_Camera`) false false)
            (`ActorComponent.SetActive` (`self.Camera_0`) true false))
          (:`B`
            (`ActorComponent.SetActive` (`self.Main_Camera`) true false)
            (`ActorComponent.SetActive` (`self.Camera_0`) false false)))))))

(event `Swoop`
  (bind _springarm (`self.SpringArm`))
  (bind _main_camera (`self.Main_Camera`))
  (bind (_returnvalue_roll _returnvalue_pitch _returnvalue_yaw) (`KismetMathLibrary.BreakRotator` (`SceneComponent.K2_GetComponentRotation` _main_camera)))
  (bind _returnvalue_roll_2 (`KismetMathLibrary.BreakRotator` (`SceneComponent.K2_GetComponentRotation` _springarm)))
  (bind (_direction _yaw _pitch) (`Timeline|Timeline_0` :!via `PlayFromStart`)
    (:`Update`
      (`SceneComponent.K2_SetWorldRotation` _springarm (`KismetMathLibrary.MakeRotator` _returnvalue_roll_2 (- _pitch 10.0) _yaw) false false)
      (`SceneComponent.K2_SetWorldRotation` _main_camera (`KismetMathLibrary.MakeRotator` _returnvalue_roll _pitch _returnvalue_yaw) false false))))

(fn `UserConstructionScript`
  (`parent.UserConstructionScript`))