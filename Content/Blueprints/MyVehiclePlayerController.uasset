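; Player controller for a kart race, managing race flow, timing, UI and saved high scores.
; Forward input on the start screen triggers the pawn's swoop, music and an animated countdown before racing begins.
; A timeline drives the race clock; stopping it fades the audio in Tick, which also restarts the level after a two-minute timeout.
; SaveGame rebuilds the five-entry leaderboard by inserting the new time ahead of slower ones.
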(event `self.ReceiveBeginPlay`
  (`AudioComponent.Stop` (`self.Audio`)))

(event `self.StartRaceTime`
  (`self.LoadGame`)
  (bind (_direction _time) (`Timeline|GameTimeline` :!via `PlayFromStart` :!label _label)
    (:`Update`
      (bind _output_get (set `self.RaceTime` _time))
      (set `self.RaceTimeText` (`self.TimeToText` _output_get)))))

(event `self.StopRaceTime`
  (set `self.FadeOutSound` true)
  (goto _label :!via `Stop`))

(event `self.SaveGameCheck`
  (bind _returnvalue (`GameplayStatics.DoesSaveGameExist` "Save"))
  (if _returnvalue
    (`self.LoadGame`)
    (else
      (bind _returnvalue_2 (`GameplayStatics.CreateSaveGameObject` "/Game/Blueprints/MySaveGame.MySaveGame_C"))
      (`GameplayStatics.SaveGameToSlot` _returnvalue_2 "Save"))))

(event `self.ShowMenu`
  (bind _asbp_kart_pawn_player (cast `/Game/Blueprints/BP_KartPawnPlayer` (`GameplayStatics.GetPlayerPawn` 0)))
  (`/Game/Blueprints/BP_KartPawnBase.On Respawn` :`self` _asbp_kart_pawn_player :`NewLocation` (0.0 0.0 100.0))
  (bind _asui (cast `/Game/Blueprints/UI` (`self.Widget`)))
  (`Widget.SetVisibility` (`/Game/Blueprints/UI.OutRace` _asui) "Visible")
  (`Widget.SetVisibility` (`/Game/Blueprints/UI.PlayerName` _asui) "Visible")
  (set `self.bShowMouseCursor` true))

(event `InputAction|Reset`
  (params (Key :type "Key Structure"))
  (:`Pressed`
    (`GameplayStatics.OpenLevel` "City")))

(event `InputAxis|Forward` :consume false
  (params (AxisValue :type "Float (single-precision)"))
  (bind _asui (cast `/Game/Blueprints/UI` (`self.Widget`) :!pure true))
  (bind _counter (`/Game/Blueprints/UI.Counter` _asui))
  (bind _start (`/Game/Blueprints/UI.Start` _asui))
  (if (and (> AxisValue 0.0) (not (`self.IsRacing`)) (`|EnumEquality` (`Widget.GetVisibility` _start) "Visible"))
    (`/Engine/EditorBlueprintResources/StandardMacros.DoOnce` false :!label _label_2
      (:`Completed`
        (`Widget.SetVisibility` _start "Collapsed")
        (`Widget.SetVisibility` (`/Game/Blueprints/UI.OutRace` _asui) "Collapsed")
        (`Widget.SetVisibility` (`/Game/Blueprints/UI.PlayerName` _asui) "Collapsed")
        (`|ExecutionSequence`
          (:`then_0`
            (`/Game/Blueprints/BP_KartPawnPlayer.Swoop` (cast `/Game/Blueprints/BP_KartPawnPlayer` (`GameplayStatics.GetPlayerPawn` 0) :!pure true))
            (`AudioComponent.Play` (`self.Audio`) 0.0))
          (:`then_1`
            (`KismetSystemLibrary.Delay` 2.0)
            (`Widget.SetVisibility` _counter "Visible")
            (`self.Text` "3")
            (`self.Text` "2")
            (`self.Text` "1")
            (`self.Text` "GO!")
            (`Widget.SetVisibility` _counter "Collapsed")
            (set `self.IsRacing` true)
            (`self.StartGameSetup`)
            (set `self.bShowMouseCursor` false)
            (goto _label_2 :!via `Reset`)))))))

(event `self.LoadGame`
  (bind _returnvalue (`GameplayStatics.LoadGameFromSlot` "Save"))
  (bind _asmy_save_game (cast `/Game/Blueprints/MySaveGame` _returnvalue))
  (bind _output_time (break `/Game/Blueprints/HighScore` (`|GetArrayItem` (`/Game/Blueprints/MySaveGame.Score` _asmy_save_game) 4)))
  (set `self.WorstRaceTime` _output_time))

(event `self.SaveGame`
  (bind _racetime (`self.RaceTime`))
  (bind _temp (`self.temp`))
  (bind _temp_2 (`self.temp`))
  (bind _returnvalue (`GameplayStatics.LoadGameFromSlot` "Save"))
  (bind _asmy_save_game (cast `/Game/Blueprints/MySaveGame` _returnvalue))
  (for _array_element (`/Game/Blueprints/MySaveGame.Score` _asmy_save_game)
    (`|ExecutionSequence`
      (:`then_0`
        (if (> (`.Time_2_86BB0A2D428EAF079A51C6AFE7C992E2` (break `/Game/Blueprints/HighScore` _array_element)) _racetime)
          (`KismetArrayLibrary.Array_AddUnique` _temp (make `/Game/Blueprints/HighScore` _racetime (`self.PlayerName`)))))
      (:`then_1`
        (`KismetArrayLibrary.Array_Add` _temp _array_element))))
  (bind _returnvalue_2 (`GameplayStatics.CreateSaveGameObject` "/Game/Blueprints/MySaveGame.MySaveGame_C"))
  (`KismetArrayLibrary.Array_Remove` _temp_2 5)
  (set `/Game/Blueprints/MySaveGame.Score` _temp_2 _returnvalue_2)
  (`GameplayStatics.SaveGameToSlot` _returnvalue_2 "Save")
  (`KismetArrayLibrary.Array_Clear` (`self.temp`)))

(event `self.ReceiveTick`
  (params (DeltaSeconds :type "Float (single-precision)"))
  (bind _audio (`self.Audio`))
  (bind _returnvalue (- (`AudioComponent.VolumeMultiplier` _audio) (/ DeltaSeconds 4.0)))
  (`|ExecutionSequence`
    (:`then_0`
      (if (`self.FadeOutSound`)
        (if (> _returnvalue 0.0)
          (`AudioComponent.SetVolumeMultiplier` _audio _returnvalue)
          (else
            (`AudioComponent.Stop` _audio)
            (`AudioComponent.SetVolumeMultiplier` _audio 0.25)
            (set `self.FadeOutSound` false)))))
    (:`then_1`
      (if (> (`self.RaceTime`) 120.0)
        (`/Engine/EditorBlueprintResources/StandardMacros.DoOnce` false
          (:`Completed`
            (bind _asui (cast `/Game/Blueprints/UI` (`self.Widget`)))
            (`Widget.SetVisibility` (`/Game/Blueprints/UI.Fail` _asui) "Visible")
            (`KismetSystemLibrary.Delay` 1.0)
            (`TextBlock.SetText` (`/Game/Blueprints/UI.FailTime` _asui) "Restart in 2...")
            (`KismetSystemLibrary.Delay` 1.0)
            (`TextBlock.SetText` (`/Game/Blueprints/UI.FailTime` _asui) "Restart in 1...")
            (`KismetSystemLibrary.Delay` 1.0)
            (`GameplayStatics.OpenLevel` "City")))))))

(event `Key|O`
  (params (Key :type "Key Structure"))
  (:`Pressed`
    (`/Engine/EditorBlueprintResources/StandardMacros.FlipFlop`
      (:`A`
        (bind _asui (cast `/Game/Blueprints/UI` (`self.Widget`)))
        (`Widget.SetVisibility` (`/Game/Blueprints/UI.Options` _asui) "Visible"))
      (:`B`
        (bind _asui_2 (cast `/Game/Blueprints/UI` (`self.Widget`)))
        (`Widget.SetVisibility` (`/Game/Blueprints/UI.Options` _asui_2) "Collapsed")))))

(fn `Sort`
  (params (TimeArray :type "Array of Float (double-precision)") (NameArray :type "Array of String"))
  (returns (Times :type "Array of Float (double-precision)") (Names :type "Array of String"))
  (locals (UnsortedTime :type "Array of Float (double-precision)") (UnsortedNames :type "Array of String") (SortedTime :type "Array of Float (double-precision)") (SortedNames :type "Array of String"))
  (bind _unsortedtime (`local.UnsortedTime`))
  (bind _sortedtime (`local.SortedTime`))
  (bind _sortednames (`local.SortedNames`))
  (bind (_indexofminvalue _minvalue) (`KismetMathLibrary.MinOfFloatArray` _unsortedtime))
  (set `local.UnsortedTime` TimeArray)
  (set `local.UnsortedNames` NameArray)
  (while (> (`KismetArrayLibrary.Array_Length` (`local.UnsortedTime`)) 0)
    (`KismetArrayLibrary.Array_Add` (`local.SortedTime`) _minvalue)
    (`KismetArrayLibrary.Array_Remove` _unsortedtime _indexofminvalue)
    (`KismetArrayLibrary.Array_Add` (`local.SortedNames`) (`|GetArrayItem` (`local.UnsortedNames`) _indexofminvalue)))
  (`KismetArrayLibrary.Array_Remove` _sortedtime (`KismetArrayLibrary.Array_LastIndex` _sortedtime))
  (`KismetArrayLibrary.Array_Remove` _sortednames (`KismetArrayLibrary.Array_LastIndex` _sortednames))
  (return (`local.SortedTime`) (`local.SortedNames`)))

(fn `UserConstructionScript`)