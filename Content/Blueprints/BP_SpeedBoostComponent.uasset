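; Speed boost component that lets its owning actor act as a boost trigger for karts.
; On BeginPlay it binds to the overlap events of the owner's primitive component and notifies any overlapping BP_KartPawnBase when the boost begins or ends.
; A DoOnce with no reset limits the begin call to the first kart overlap, while the end call fires on every exit.
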(event `self.ReceiveBeginPlay`
  (bind _returnvalue (`Actor.GetComponentByClass` (`self.GetOwner`) "/Script/Engine.PrimitiveComponent"))
  (`/Engine/EditorBlueprintResources/StandardMacros.IsValid` _returnvalue
    (:`Is Valid`
      (add `PrimitiveComponent.OnComponentBeginOverlap` _returnvalue (delegate `OnComponentBeginOverlap`))
      (add `PrimitiveComponent.OnComponentEndOverlap` _returnvalue (delegate `OnComponentEndOverlap`)))))

(event `OnComponentEndOverlap`
  (params (OverlappedComponent :type "PrimitiveComponent Object Reference") (OtherActor :type "Actor Object Reference") (OtherComp :type "PrimitiveComponent Object Reference") (OtherBodyIndex :type Integer))
  (bind _asbp_kart_pawn_base (cast `/Game/Blueprints/BP_KartPawnBase` OtherActor))
  (`/Game/Blueprints/BP_KartPawnBase.On Speed Boost End` _asbp_kart_pawn_base))

(event `OnComponentBeginOverlap`
  (params (OverlappedComponent :type "PrimitiveComponent Object Reference") (OtherActor :type "Actor Object Reference") (OtherComp :type "PrimitiveComponent Object Reference") (OtherBodyIndex :type Integer) (bFromSweep :type Boolean) (SweepResult :type "HitResult Structure (by ref)"))
  (bind _asbp_kart_pawn_base (cast `/Game/Blueprints/BP_KartPawnBase` OtherActor))
  (`/Engine/EditorBlueprintResources/StandardMacros.DoOnce` false
    (:`Completed`
      (`/Game/Blueprints/BP_KartPawnBase.On Speed Boost Begin` _asbp_kart_pawn_base))))