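; Speed boost volume actor whose Blueprint graphs handle only the animated color of its arrow mesh, with no boost logic.
; The construction script creates two dynamic instances of the arrow material, one for each of the first two static mesh material slots.
; On BeginPlay, the Alpha timeline starts and writes its Color track into both instances' Color parameter on every update.
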(event `self.ReceiveBeginPlay`
  (bind (_direction _color) (`Timeline|Alpha` :!via `PlayFromStart`)
    (:`Update`
      (bind _returnvalue (`KismetMathLibrary.Conv_VectorToLinearColor` _color))
      (`MaterialInstanceDynamic.SetVectorParameterValue` (`self.Material0`) "Color" _returnvalue)
      (`MaterialInstanceDynamic.SetVectorParameterValue` (`self.Material1`) "Color" _returnvalue))))

(fn `UserConstructionScript`
  (bind _returnvalue (`PrimitiveComponent.CreateDynamicMaterialInstance` (`self.StaticMesh`) 0 "/Game/Materials/Arrow_Mat.Arrow_Mat"))
  (set `self.Material0` _returnvalue)
  (bind _returnvalue_2 (`PrimitiveComponent.CreateDynamicMaterialInstance` (`self.StaticMesh`) 1 "/Game/Materials/Arrow_Mat.Arrow_Mat"))
  (set `self.Material1` _returnvalue_2))